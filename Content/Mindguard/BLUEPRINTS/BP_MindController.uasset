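; BP_MindController is an AI controller that runs the BT_Mind behavior tree for the Mind.
; On BeginPlay it starts the tree, sets the IsPlayerActive blackboard key true and IsMoving false, then calls SetPlayerActive.
; SetPlayerActive is an empty stub, and the logic to cache the player and bind it to OnPlayerSwitch is disconnected, so player switches never update the blackboard.
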(event Custom|SetPlayerActive
  ;[1 1 1] Set AI to behaviour tree and its values
  ;;[1 1 1] Switch Mind activity bool
)

(event EventBeginPlay
  ;[1 1 1] Set AI to behaviour tree and its values
  (AI|RunBehaviorTree "/Game/Mindguard/AI/BT_Mind.BT_Mind")
  ;;[1 1 1] Switch Mind activity bool
  (AI|Components|Blackboard|SetValueasBool (Variables|Default|GetBlackboard) (Utilities|Name|MakeLiteralName "IsPlayerActive") true)
  ;;[1 1 1] set default movement to false
  (AI|Components|Blackboard|SetValueasBool (Variables|Default|GetBlackboard) (Utilities|Name|MakeLiteralName "IsMoving") false)
  ;;[1 1 1] Default activity
  (CallFunction|SetPlayerActive))

(fn ConstructionScript)