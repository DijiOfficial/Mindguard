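; Player pawn for step-based movement, with an active/inactive switch for player swapping and shield pick-up or drop.
; On possession it binds to BP_PlayerController's move, rotate, switch and interact events, accepting moves and 90-degree turns only when active and idle.
; Tick sweeps each fixed-distance step, then snaps to the target.
; Capsule hits try pushing BP_Moveable_AC objects; failed pushes, other hits and shield-box overlaps snap the pawn back to its starting position.
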(event OnComponentHit(CapsuleComponent)
  (params (HitComponent :type Primitive%20Component%20Object%20Reference) (OtherActor :type Actor%20Object%20Reference) (OtherComp :type Primitive%20Component%20Object%20Reference) (NormalImpulse :type Vector :default "0, 0, 0") (Hit :type Hit%20Result%20Structure%20%28by%20ref%29))
  (bind _returnvalue (Actor|GetComponentbyClass OtherActor "/Game/Mindguard/BLUEPRINTS/Components_Interfaces/BP_Moveable_AC.BP_Moveable_AC_C"))
  ;[1 1 1] Handle Collision
  (Utilities|IsValid OtherActor
    (:Is%20Valid
      (Utilities|IsValid _returnvalue
        (:Is%20Valid
          (bind _ismovementvalid (Default|MoveActor _returnvalue (Variables|Movement|GetDesiredDirection)))
          ;;[1 1 1] Object cannot be moved
          (if (not _ismovementvalid)
            ;;[1 1 1] If player is colliding disable movement and reset location
            (if (Variables|Movement|GetIsMoving) :!label _label
              (Variables|Movement|SetIsMoving false)
              (Transformation|SetActorLocation (Variables|Movement|GetOriginalLocation) false false))))
        (:Is%20Not%20Valid
          (goto _label))))
    (:Is%20Not%20Valid
      (goto _label))))

(event OnComponentBeginOverlap(ShieldCollisionBox)
  (params (OverlappedComponent :type Primitive%20Component%20Object%20Reference) (OtherActor :type Actor%20Object%20Reference) (OtherComp :type Primitive%20Component%20Object%20Reference) (OtherBodyIndex :type Integer) (bFromSweep :type Boolean) (SweepResult :type Hit%20Result%20Structure%20%28by%20ref%29))
  ;[1 0.02643 0] Temporary collision with shield until I figure out better collision?
  (Utilities|Casting|CastToBP_Shield OtherActor)
  ;[1 1 1] Handle Collision
  ;;[1 1 1] If player is colliding disable movement and reset location
  (if (Variables|Movement|GetIsMoving)
    (Variables|Movement|SetIsMoving false)
    (Transformation|SetActorLocation (Variables|Movement|GetOriginalLocation) false false)))

(event Custom|SetTargetRotation
  (params (RotateRight :type Boolean))
  ;[1 1 1] Player Rotation
  (if (CallFunction|IsPlayerMoving)
    (if RotateRight
      (Variables|Movement|SetRotationAngle 9e+01)
      (else
        (Variables|Movement|SetRotationAngle -9e+01)))
    (Transformation|SetWorldRotation (Variables|Character|GetMesh) (Math|Rotator|MakeRotator 0.0 0.0 (+ (.yaw (Transformation|GetWorldRotation (Variables|Character|GetMesh))) (Variables|Movement|GetRotationAngle))) false false)))

(event Custom|SwitchPlayer
  ;[1 1 1] PlayerSwitch
  (Utilities|FlowControl|DoOnce false :!label _label
    (:Completed
      (Utilities|FlowControl|Sequence
        (:then_0
          (Variables|PlayerControl|SetIsActive (not (Variables|PlayerControl|GetIsActive)))
          (Default|CallOnPlayerSwitch))
        (:then_1
          (Utilities|FlowControl|Delay (Variables|PlayerControl|GetSwitchDelay))
          (goto _label Reset))))))

(event Custom|InteractWithShield
  (bind _overlappingactors (Collision|GetOverlappingActors "/Game/Mindguard/BLUEPRINTS/Actors/BP_Shield.BP_Shield_C" :!class /Script/Engine.Actor))
  (if (Variables|Shield|GetHasShield)
    (Class|BPIPickeable|Drop(Message) _overlappingactors)
    (Variables|Shield|SetHasShield false)
    (else
      (Class|BPIPickeable|PickUp(Message) _overlappingactors (Variables|Default|GetShieldSocket))
      (Variables|Shield|SetHasShield true))))

(event Custom|MovePlayer
  (params (TargetLocation :type Vector))
  (bind _returnvalue (Transformation|GetActorLocation))
  ;[1 1 1] Set Player to move
  (if (CallFunction|IsPlayerMoving)
    (Variables|Movement|SetDesiredDirection (Math|Vector|Normalize TargetLocation))
    (Variables|Movement|SetMoveDistanceLeft 1e+02)
    (Variables|Movement|SetOriginalLocation _returnvalue)
    (Variables|Movement|SetTargetLocation (+ _returnvalue TargetLocation))
    (Animation|Montage|PlayMontage (Variables|Character|GetMesh) "/Game/ShooterMannequin/Animations/AM_ThirdPersonWalk.AM_ThirdPersonWalk" 2.5
      (:then
        (Variables|Movement|SetIsMoving true)))))

(event EventPossessed
  (params (NewController :type Controller%20Object%20Reference))
  (bind _returnvalue (Pawn|GetController))
  (bind _asbp_player_controller (Utilities|Casting|CastToBP_PlayerController _returnvalue))
  ;[1 1 1] Player Listeners evetns (perhaps move to construction script)
  (EventDispatchers|BindEventtoOnRotationInput _asbp_player_controller (delegate Custom|SetTargetRotation))
  (EventDispatchers|BindEventtoOnMovementInput _asbp_player_controller (delegate Custom|MovePlayer))
  (EventDispatchers|BindEventtoOnSwitchInput _asbp_player_controller (delegate Custom|SwitchPlayer))
  (EventDispatchers|AssignOnInteractInput _asbp_player_controller (delegate Custom|InteractWithShield)))

(event EventTick
  (params (DeltaSeconds :type Float%20%28single-precision%29))
  (bind _movement_speed (Variables|Movement|GetMOVEMENT_SPEED))
  (bind _returnvalue (* DeltaSeconds _movement_speed))
  ;[1 1 1] Player Movement
  (if (Variables|PlayerControl|GetIsActive)
    (if (Variables|Movement|GetIsMoving)
      ;;[1 1 1] Move Pawn
      (Transformation|AddActorWorldOffset (* (Variables|Movement|GetDesiredDirection) _returnvalue) true)
      (bind _output_get (Variables|Movement|SetMoveDistanceLeft (- (Variables|Movement|GetMoveDistanceLeft) _returnvalue)))
      ;;[1 1 1] Disable Movement and make sure actor is in the desired location
      (if (and (<= _output_get 0.0) (Variables|Movement|GetIsMoving))
        (Variables|Movement|SetIsMoving false)
        (Transformation|SetActorLocation (Variables|Movement|GetTargetLocation) false false)
        (Animation|StopAnimMontage "/Game/ShooterMannequin/Animations/AM_ThirdPersonWalk.AM_ThirdPersonWalk")))))

(fn ConstructionScript
  (|CallParentFunction))

(fn IsPlayerActive
  (return (Variables|PlayerControl|GetIsActive)))

(fn IsPlayerMoving
  (return (and (Variables|PlayerControl|GetIsActive) (not (Variables|Movement|GetIsMoving)))))