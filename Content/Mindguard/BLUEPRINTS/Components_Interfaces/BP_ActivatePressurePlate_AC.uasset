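; Actor component that lets its owning actor activate pressure plates by overlapping them.
; On BeginPlay it binds to the owner's actor begin and end overlap events.
; When the other actor implements BPI_Interact, it sends InteractMessage on overlap begin and EndInteractMessage on overlap end, so any interactable can respond.
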(event Custom|OnActorBeginOverlap_Event
  (params (OverlappedActor :type Actor%20Object%20Reference) (OtherActor :type Actor%20Object%20Reference))
  ;[1 1 1] Interact with Pressure Plate when overlapping
  (if (Utilities|DoesObjectImplementInterface OtherActor "/Game/Mindguard/Blueprints/Components_Interfaces/BPI_Interact.BPI_Interact_C")
    (Class|BPIInteract|Interact(Message) OtherActor)))

(event Custom|OnActorEndOverlap_Event
  (params (OverlappedActor :type Actor%20Object%20Reference) (OtherActor :type Actor%20Object%20Reference))
  ;[1 1 1] Stop Interacting with it
  (if (Utilities|DoesObjectImplementInterface OtherActor "/Game/Mindguard/Blueprints/Components_Interfaces/BPI_Interact.BPI_Interact_C")
    (Class|BPIInteract|EndInteract(Message) OtherActor)))

(event EventBeginPlay
  (bind _returnvalue (Components|GetOwner))
  ;[1 1 1] Bind Overlap Events to trigger pressure plates events
  (EventDispatchers|AssignOnActorBeginOverlap _returnvalue (delegate Custom|OnActorBeginOverlap_Event))
  (EventDispatchers|AssignOnActorEndOverlap _returnvalue (delegate Custom|OnActorEndOverlap_Event)))