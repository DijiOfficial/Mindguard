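; BP_Moveable_AC is an actor component that moves its owner in 100-unit horizontal steps.
; MoveActor plays a whoosh and sweeps one step along the given direction, snapping back if blocked and returning whether it succeeded.
; OriginalTransform stores the location at BeginPlay but is overwritten by every MoveActor call, so Reset restores the position before the latest move attempt.
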(event Custom|Reset
  ;[1 1 1] Reset
  (Transformation|SetActorLocation (Components|GetOwner) (Variables|Transform|GetOriginalTransform) false false))

(event EventBeginPlay
  ;[1 1 1] Reset
  (Variables|Transform|SetOriginalTransform (Transformation|GetActorLocation (Components|GetOwner))))

(fn MoveActor
  (params (Direction :type Vector :default "0, 0, 0"))
  (bind _returnvalue (Components|GetOwner))
  (bind _returnvalue_2 (Transformation|GetActorLocation _returnvalue))
  ;[1 1 1] Move Actor if no collision is deteced and return collision result
  (bind _output_get (Variables|Transform|SetOriginalTransform _returnvalue_2))
  (Audio|PlaySoundatLocation "/Game/Mindguard/Audio/SFX/A_Whoosh.A_Whoosh" _output_get "0, 0, 0" 1.0 1.0 0.0 0 0 0 0)
  (bind _sweephitresult (Transformation|SetActorLocation _returnvalue (+ (* Direction "100.000000,100.000000,0.000000") _returnvalue_2) true false))
  (if (.bblockinghit _sweephitresult)
    (Transformation|SetActorLocation _returnvalue (Variables|Transform|GetOriginalTransform) false false))
  (return (not (.bblockinghit _sweephitresult))))