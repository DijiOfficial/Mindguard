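; Player controller for Mindguard that sets up Enhanced Input and the HUD, and relays player input through event dispatchers.
; Movement input becomes 100-unit axis-aligned offsets, while rotation, control switch and interact inputs are broadcast directly.
; Camera switch toggles possession between the player character and a spectator camera spawned at the character's camera.
; Pause input toggles the pause menu, game pause, cursor and input mode.
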(event Input|EnhancedActionEvents|EnhancedInputActionIA_PlayerMovement
  (params (ActionValue :type Vector%202D%20Structure) (ElapsedSeconds :type Float%20%28double-precision%29) (TriggeredSeconds :type Float%20%28double-precision%29) (InputAction :type Input%20Action%20Object%20Reference :default "/Game/Mindguard/Input/ACTIONS/IA_PlayerMovement.IA_PlayerMovement"))
  (bind _returnvalue (Class|KismetMathLibrary|FCeil64 (.y ActionValue)))
  (bind _returnvalue_2 (Class|KismetMathLibrary|FCeil64 (.x ActionValue)))
  ;[0 1 0] Handle Movement Input
  (:Started
    (Utilities|FlowControl|Sequence
      (:then_0
        (if (!= _returnvalue_2 0)
          (if (> _returnvalue_2 0)
            (Variables|Movement|SetTargetLocation "0.000000,100.000000,0.000000")
            (else
              (Variables|Movement|SetTargetLocation "0.000000,-100.000000,0.000000")))
          (Default|CallOnMovementInput (Variables|Movement|GetTargetLocation) :!label _label)))
      (:then_1
        (if (!= _returnvalue 0)
          (if (> _returnvalue 0)
            (Variables|Movement|SetTargetLocation "100.000000,0.000000,0.000000")
            (goto _label)
            (else
              (Variables|Movement|SetTargetLocation "-100.000000,0.000000,0.000000")
              (goto _label))))))))

(event Input|EnhancedActionEvents|EnhancedInputActionIA_SwitchControl
  (params (ActionValue :type Boolean) (ElapsedSeconds :type Float%20%28double-precision%29) (TriggeredSeconds :type Float%20%28double-precision%29) (InputAction :type Input%20Action%20Object%20Reference :default "/Game/Mindguard/Input/ACTIONS/IA_SwitchControl.IA_SwitchControl"))
  ;[1 1 1] Call Player Rotation, Switch and Interaction event
  (Default|CallOnSwitchInput))

(event Input|EnhancedActionEvents|EnhancedInputActionIA_RotateRight
  (params (ActionValue :type Boolean) (ElapsedSeconds :type Float%20%28double-precision%29) (TriggeredSeconds :type Float%20%28double-precision%29) (InputAction :type Input%20Action%20Object%20Reference :default "/Game/Mindguard/Input/ACTIONS/IA_RotateRight.IA_RotateRight"))
  ;[1 1 1] Call Player Rotation, Switch and Interaction event
  (:Started
    (Default|CallOnRotationInput true)))

(event Input|EnhancedActionEvents|EnhancedInputActionIA_RotateLeft
  (params (ActionValue :type Boolean) (ElapsedSeconds :type Float%20%28double-precision%29) (TriggeredSeconds :type Float%20%28double-precision%29) (InputAction :type Input%20Action%20Object%20Reference :default "/Game/Mindguard/Input/ACTIONS/IA_RotateLeft.IA_RotateLeft"))
  ;[1 1 1] Call Player Rotation, Switch and Interaction event
  (:Started
    (Default|CallOnRotationInput false)))

(event Input|EnhancedActionEvents|EnhancedInputActionIA_Interact
  (params (ActionValue :type Boolean) (ElapsedSeconds :type Float%20%28double-precision%29) (TriggeredSeconds :type Float%20%28double-precision%29) (InputAction :type Input%20Action%20Object%20Reference :default "/Game/Mindguard/Input/ACTIONS/IA_Interact.IA_Interact"))
  ;[1 1 1] Call Player Rotation, Switch and Interaction event
  (:Started
    (Default|CallOnInteractInput)))

(event Input|EnhancedActionEvents|EnhancedInputActionIA_Pause
  (params (ActionValue :type Boolean) (ElapsedSeconds :type Float%20%28double-precision%29) (TriggeredSeconds :type Float%20%28double-precision%29) (InputAction :type Input%20Action%20Object%20Reference :default "/Game/Mindguard/Input/ACTIONS/IA_Pause.IA_Pause"))
  (bind _self self)
  ;[1 1 1] Pausing input
  (:Started
    (if (Game|IsGamePaused)
      (bind _foundwidgets (Widget|GetAllWidgetsOfClass "/Game/Mindguard/UI/W_PauseMenu.W_PauseMenu_C" true))
      (Widget|RemovefromParent _foundwidgets)
      (Variables|Default|SetbShowMouseCursor false)
      (Game|SetGamePaused false)
      (Input|SetInputModeGameOnly _self true)
      ;[1 1 1] If controls hud delete it too
      (bind _foundwidgets_2 (Widget|GetAllWidgetsOfClass "/Game/Mindguard/UI/W_Controls.W_Controls_C" true))
      (Widget|RemovefromParent _foundwidgets_2)
      (else
        (bind _returnvalue (UserInterface|CreateWidget "/Game/Mindguard/UI/W_PauseMenu.W_PauseMenu_C"))
        (UserInterface|Viewport|AddtoViewport _returnvalue 0)
        (Variables|Default|SetbShowMouseCursor true)
        (Input|SetInputModeGameandUI _self 0 "DoNotLock" true false)
        (Game|SetGamePaused true)))))

(event Input|EnhancedActionEvents|EnhancedInputActionIA_SwitchCamera
  (params (ActionValue :type Boolean) (ElapsedSeconds :type Float%20%28double-precision%29) (TriggeredSeconds :type Float%20%28double-precision%29) (InputAction :type Input%20Action%20Object%20Reference :default "/Game/Mindguard/Input/ACTIONS/IA_SwitchCamera.IA_SwitchCamera"))
  ;[1 1 1] On Camera Switch Input
  (:Started
    (Default|CallOnCameraSwitchInput)
    (if (not (Variables|Default|GetIsControllingPlayer))
      ;;[1 1 1] If controlling spectator camera, get the player and posses it and destory the spectator
      (bind _outactors (Actor|GetAllActorsOfClass "/Game/Mindguard/Blueprints/Characters/BP_PlayerCharacter.BP_PlayerCharacter_C"))
      (Pawn|Possess (Utilities|Array|Get(acopy) _outactors))
      (bind _outactors_2 (Actor|GetAllActorsOfClass "/Game/Mindguard/Blueprints/Characters/BP_SpectatorCamera.BP_SpectatorCamera_C"))
      (Actor|DestroyActor _outactors_2)
      (Variables|Default|SetIsControllingPlayer true)
      (else
        ;;[1 1 1] If Controlling player create spectator and posses it
        (bind _returnvalue (Game|SpawnActorfromClass "/Game/Mindguard/Blueprints/Characters/BP_SpectatorCamera.BP_SpectatorCamera_C" (Transformation|GetWorldTransform (Variables|/Game/Mindguard/Blueprints/Characters/BP_PlayerCharacter.BP_PlayerCharacter_C|GetCamera (.AsBP%20Player%20Character (Utilities|Casting|CastToBP_PlayerCharacter (Pawn|GetControlledPawn))))) "AdjustIfPossibleButAlwaysSpawn" "MultiplyWithRoot" 0 0))
        (Pawn|Possess _returnvalue)
        (Variables|Default|SetIsControllingPlayer false)))))

(event EventBeginPlay
  (bind _returnvalue (PlayerController|LocalPlayerSubsystems|GetEnhancedInputLocalPlayerSubsystem))
  (Utilities|FlowControl|Sequence
    (:then_0
      ;[1 1 1] Enable the Player Input mapping context
      (Utilities|IsValid _returnvalue
        (:Is%20Valid
          (Input|AddMappingContext _returnvalue "/Game/Mindguard/Input/MAPPINGS/IMC_Player.IMC_Player" 0 "(bIgnoreAllPressedKeysUntilRelease=True,bForceImmediately=False,bNotifyUserSettings=False)"))))
    (:then_1
      ;[1 1 1] Hud Creation
      (bind _returnvalue_2 (UserInterface|CreateWidget "/Game/Mindguard/UI/W_HUD.W_HUD_C" self))
      (UserInterface|Viewport|AddtoViewport _returnvalue_2 0))))

(fn ConstructionScript)