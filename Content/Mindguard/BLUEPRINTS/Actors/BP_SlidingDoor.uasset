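; BP_SlidingDoor is a door actor that slides open and closed as triggers interact with it.
; Open calls increment a trigger counter and play a timeline, while close calls decrement it and reverse the timeline only at zero.
; The timeline lerps the Visual component's relative location from Origin, cached as the actor's location in the Construction Script, to Origin plus a final offset.
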(event Custom|OPEN%20GNE%20GNOOOR
  (bind _origin (Variables|LocationInfo|GetOrigin))
  ;[1 1 1] Latch for opening closing the door based on triggers interacting with it
  (Variables|Parameter|SetTriggerCounter (+ (Variables|Parameter|GetTriggerCounter) 1))
  (bind _opentrack (Timeline|OpenDoor Play)
    (:Update
      ;[1 1 1] Set Door Relative position based on timeline timer
      (Transformation|SetRelativeLocation (Variables|Default|GetVisual) (Math|Vector|Lerp(Vector) _origin (+ _origin (Variables|LocationInfo|GetFINAL_VERTICAL_OFFSET)) _opentrack) false false))))

(event Custom|CloseDoor
  (bind _origin (Variables|LocationInfo|GetOrigin))
  ;[1 1 1] Latch for opening closing the door based on triggers interacting with it
  (bind _output_get (Variables|Parameter|SetTriggerCounter (- (Variables|Parameter|GetTriggerCounter) 1)))
  (if (== _output_get 0)
    (bind _opentrack (Timeline|OpenDoor Reverse)
      (:Update
        ;[1 1 1] Set Door Relative position based on timeline timer
        (Transformation|SetRelativeLocation (Variables|Default|GetVisual) (Math|Vector|Lerp(Vector) _origin (+ _origin (Variables|LocationInfo|GetFINAL_VERTICAL_OFFSET)) _opentrack) false false)))))

(fn ConstructionScript
  ;[1 1 1] Set the origin once
  (Variables|LocationInfo|SetOrigin (Transformation|GetActorLocation)))