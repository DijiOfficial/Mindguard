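; BP_PickeableInfo is an info label actor that shows configurable floating text in the world, by its name for pickable items.
; Construction applies the text content and height offset, and box overlaps with BP_PlayerCharacter toggle its visibility unless ALWAYSACTIVE keeps it shown.
; While displayable, Tick rotates the text toward the player camera.
; EnableTextBool and DisableTextBool functions switch the display directly, without checking the always-active flag.
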(event OnComponentBeginOverlap(Box)
  (params (OverlappedComponent :type Primitive%20Component%20Object%20Reference) (OtherActor :type Actor%20Object%20Reference) (OtherComp :type Primitive%20Component%20Object%20Reference) (OtherBodyIndex :type Integer) (bFromSweep :type Boolean) (SweepResult :type Hit%20Result%20Structure%20%28by%20ref%29))
  ;[1 1 1] Change display settings based on player overlap
  (if (not (Variables|Parameters|GetALWAYS_ACTIVE))
    (Utilities|Casting|CastToBP_PlayerCharacter OtherActor)
    (Variables|Visibility|SetCanDisplay true)
    (Rendering|SetVisibility (Variables|Default|GetTextRender) true false)))

(event OnComponentEndOverlap(Box)
  (params (OverlappedComponent :type Primitive%20Component%20Object%20Reference) (OtherActor :type Actor%20Object%20Reference) (OtherComp :type Primitive%20Component%20Object%20Reference) (OtherBodyIndex :type Integer))
  ;[1 1 1] Change display settings based on player overlap
  (if (not (Variables|Parameters|GetALWAYS_ACTIVE))
    (Utilities|Casting|CastToBP_PlayerCharacter OtherActor)
    (Variables|Visibility|SetCanDisplay false)
    (Rendering|SetVisibility (Variables|Default|GetTextRender) false false)))

(event EventTick
  (params (DeltaSeconds :type Float%20%28single-precision%29))
  (bind _textrender (Variables|Default|GetTextRender))
  ;[1 1 1] Set rotation towards camera if can be displayed
  (if (Variables|Visibility|GetCanDisplay)
    (Transformation|SetWorldRotation _textrender (Math|Rotator|FindLookatRotation (Transformation|GetWorldLocation _textrender) (Camera|GetCameraLocation (Game|GetPlayerCameraManager 0))) false false)))

(event EventBeginPlay
  (bind _always_active (Variables|Parameters|GetALWAYS_ACTIVE))
  ;[1 1 1] Set Visibilty to false
  (Rendering|SetVisibility (Variables|Default|GetTextRender) _always_active false)
  (Variables|Visibility|SetCanDisplay _always_active))

(fn ConstructionScript
  (bind _textrender (Variables|Default|GetTextRender))
  (Transformation|SetRelativeLocation _textrender (Math|Vector|MakeVector 0.0 0.0 (Variables|Parameters|GetTextOffsetZ)) false false)
  (Rendering|Components|TextRender|SetText _textrender (Variables|Parameters|GetTextContent)))

(fn DisableTextBool
  (Variables|Visibility|SetCanDisplay false)
  (Rendering|SetVisibility (Variables|Default|GetTextRender) false false))

(fn EnableTextBool
  (Variables|Visibility|SetCanDisplay true)
  (Rendering|SetVisibility (Variables|Default|GetTextRender) true false))