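; BP_Shield is a shield actor that the player can pick up and drop.
; PickUp snaps it to the given socket component, turns off the text on its InfoBubble child actor (BP_PickeableInfo) and plays a pickup sound.
; Drop detaches it in world space, moves it to a fixed world Z height, turns the text back on and plays a drop sound.
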(event EventPickUp
  (params (Socket :type Arrow%20Component%20Object%20Reference))
  ;[1 1 1] Attach to player
  (Transformation|AttachComponentToComponent Socket "None" "SnapToTarget" "SnapToTarget" "SnapToTarget" true)
  ;;[1 1 1] Disable the text
  (bind _asbp_pickeable_info (Utilities|Casting|CastToBP_PickeableInfo (Variables|/Script/Engine.ChildActorComponent|GetChildActor (Variables|Default|GetInfoBubble))))
  (Default|DisableTextBool _asbp_pickeable_info)
  (Audio|PlaySound2D "/Game/Mindguard/Audio/SFX/A_Pickup.A_Pickup" 1.0 1.0 0.0 0 0))

(event EventDrop
  (bind _returnvalue (Transformation|GetActorLocation))
  ;[1 1 1] Detach and set Z position accordingly
  (Transformation|DetachFromActor "KeepWorld" "KeepWorld" "KeepWorld")
  (Transformation|SetActorLocation (Math|Vector|MakeVector (.x _returnvalue) (.y _returnvalue) 1e+02) false false)
  (bind _asbp_pickeable_info (Utilities|Casting|CastToBP_PickeableInfo (Variables|/Script/Engine.ChildActorComponent|GetChildActor (Variables|Default|GetInfoBubble))))
  (Default|EnableTextBool _asbp_pickeable_info)
  (Audio|PlaySound2D "/Game/Mindguard/Audio/SFX/A_Drop.A_Drop" 1.0 1.0 0.0 0 0))

(fn ConstructionScript)